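; BP_Character_2D is a 2D character Blueprint that computes its rectangular collision bounds.
; CollisionValue derives min and max edges from the actor's location and half its Width and Height, treating world Z as the 2D Y axis.
; Tick calls it every frame, printing the actor's name and color-coded bounds as debug output.
; The function returns the four edges, but Tick does not use them.
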(event `self.ReceiveTick`
  (params (DeltaSeconds :type "Float (single-precision)"))
  (`self.CollisionValue`))

(fn `CollisionValue`
  (returns (MaxX :type "Float (double-precision)") (MinX :type "Float (double-precision)") (MaxY :type "Float (double-precision)") (MinY :type "Float (double-precision)"))
  (bind _returnvalue (`self.GetTransform`))
  (bind _returnvalue_2 (/ (`self.Height`) 2.0))
  (bind _returnvalue_3 (/ (`self.Width`) 2.0))
  (bind _returnvalue_4 (+ (.x (.location _returnvalue)) _returnvalue_3))
  (bind _returnvalue_5 (- (.z (.location _returnvalue)) _returnvalue_2))
  (bind _returnvalue_6 (+ (.z (.location _returnvalue)) _returnvalue_2))
  (bind _returnvalue_7 (- (.x (.location _returnvalue)) _returnvalue_3))
  (`KismetSystemLibrary.PrintString` (`KismetSystemLibrary.GetDisplayName` self) true true (struct :`R` 0.5 :`B` 1.0 :`A` 1.0) 1.0)
  ; MaxX
  (`KismetSystemLibrary.PrintString` (`KismetStringLibrary.Concat_StrStr` "MaxX : " (`KismetStringLibrary.Conv_DoubleToString` _returnvalue_4)) true true (struct :`R` 1.0 :`G` 1.0 :`A` 1.0) 1.0)
  ; MinX
  (`KismetSystemLibrary.PrintString` (`KismetStringLibrary.Concat_StrStr` "MinX : " (`KismetStringLibrary.Conv_DoubleToString` _returnvalue_7)) true true (struct :`R` 1.0 :`G` 1.0 :`A` 1.0) 1.0)
  ; MaxY
  (`KismetSystemLibrary.PrintString` (`KismetStringLibrary.Concat_StrStr` "MaxY : " (`KismetStringLibrary.Conv_DoubleToString` _returnvalue_6)) true true (struct :`G` 1.0 :`B` 1.0 :`A` 1.0) 1.0)
  ; MinY
  (`KismetSystemLibrary.PrintString` (`KismetStringLibrary.Concat_StrStr` "MinY : " (`KismetStringLibrary.Conv_DoubleToString` _returnvalue_5)) true true (struct :`G` 1.0 :`B` 1.0 :`A` 1.0) 1.0)
  (return _returnvalue_4 _returnvalue_7 _returnvalue_6 _returnvalue_5))

(fn `UserConstructionScript`)